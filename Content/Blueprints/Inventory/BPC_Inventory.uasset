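; Inventory component that binds the pickup and inventory Enhanced Input actions.
; Pickup calls Interactable with EPickup, then debug-prints the container count and each container's slot and item data, including tags, IDs, rotation, amount and equip data.
; The inventory action calls ToggleInventory to open the inventory with a fade.
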(event `EnhancedInput|/Game/Blueprints/Input/Actions/IA_Pickup`
  (params (ActionValue :type Boolean) (ElapsedSeconds :type "Float (double-precision)") (TriggeredSeconds :type "Float (double-precision)") (InputAction :type "InputAction Object Reference" :default "/Game/Blueprints/Input/Actions/IA_Pickup.IA_Pickup"))
  (bind _containers (`self.Containers`))
  (bind _returnvalue (`KismetArrayLibrary.Array_Length` _containers))
  (:`Started`
    (`self.Interactable` "E_Pickup")
    (`KismetSystemLibrary.PrintString` (`KismetStringLibrary.Conv_IntToString` _returnvalue))
    (if (> _returnvalue 0)
      (for _array_element _containers
        (`|ExecutionSequence`
          (:`then_0`
            (bind ((`Slots` _slots) (`Items` _items)) (break `ContainerInfo` _array_element))
            (if (not (`KismetArrayLibrary.Array_IsEmpty` _slots))
              (for _array_element_2 _slots
                (bind (_slottag _parentcontaineruid _slotid _itemslotid _bisempty) (break `SlotInfo` _array_element_2))
                (`KismetSystemLibrary.PrintString` (`KismetStringLibrary.Concat_StrStr` "SlotTag:" (`KismetStringLibrary.Conv_NameToString` (`BlueprintGameplayTagLibrary.GetTagName` _slottag)) "  ParentContainerUID:" (`KismetStringLibrary.Conv_IntToString` _parentcontaineruid) "   SlotID: " (`KismetStringLibrary.Conv_IntToString` _slotid) "   ItemSlotID:" (`KismetStringLibrary.Conv_IntToString` _itemslotid) "   IsEmpty:" (`KismetStringLibrary.Conv_BoolToString` _bisempty))))))
          (:`then_1`
            (if (not (`KismetArrayLibrary.Array_IsEmpty` _items))
              (for _array_element_3 _items
                (bind (_itemid _brotated _itemamount _currentslotid _owncontaineruids _equipdata) (break `ItemInfoDef` _array_element_3))
                (`KismetSystemLibrary.PrintString` (`KismetStringLibrary.Concat_StrStr` "ItemID:" (`KismetStringLibrary.Conv_NameToString` _itemid) "  Rotated:" (`KismetStringLibrary.Conv_BoolToString` _brotated) "   ItemAmount: " (`KismetStringLibrary.Conv_IntToString` _itemamount) "  CurrentSlotID:" (`KismetStringLibrary.Conv_IntToString` _currentslotid) "  EquipData:" (`KismetSystemLibrary.GetDisplayName` _equipdata)))))))))))

(event `EnhancedInput|/Game/Blueprints/Input/Actions/IA_Inventory`
  (params (ActionValue :type Boolean) (ElapsedSeconds :type "Float (double-precision)") (TriggeredSeconds :type "Float (double-precision)") (InputAction :type "InputAction Object Reference" :default "/Game/Blueprints/Input/Actions/IA_Inventory.IA_Inventory"))
  (:`Started`
    (`self.ToggleInventory` true true)))