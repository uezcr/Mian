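; BP_PickupSpawner is a placeable placeholder that turns into a BP_PickupActor for a given ItemID at BeginPlay.
; With UpdateMeshOnConstruct set, the construction script previews the cached item's pickup mesh with an ItemID label above it.
; The authority constructs the item's equipment definition and spawns the pickup, keeping ItemAmount only for stackables and SubItems only with valid OwnInventoryData.
; The spawner then destroys itself; remote copies destroy themselves immediately.
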(event `self.ReceiveBeginPlay`
  (`/Engine/EditorBlueprintResources/ActorMacros.Switch Has Authority`
    (:`Authority`
      (set `self.ItemDefault` (`InventoryLibrary.GetDefaultIneventoryItemById` (`self.Item ID`)))
      (`|ExecutionSequence`
        (:`then_0`
          (bind _returnvalue (`|GenericCreateObject` (`.EquipmentDefinition` (break `InventoryItem` (`self.ItemDefault`)))))
          (set `self.EquipmentDef` _returnvalue))
        (:`then_1`
          (`|SpawnActorFromClass` "/Game/Blueprints/Inventory/PickupSpawner/BP_PickupActor.BP_PickupActor_C" (`self.GetTransform`) "Undefined" "MultiplyWithRoot" null (`|MakeArray`) (make `ItemInfoDef` (`self.Item ID`) false (`KismetMathLibrary.SelectInt` (`self.Item Amount`) 1 (`InventoryLibrary.IsStackable` (`self.ItemDefault`))) 0 (`|MakeArray`) (`self.EquipmentDef`)) (select `bool` (`KismetSystemLibrary.IsValid` (`.OwnInventoryData` (break `InventoryItem` (`self.ItemDefault`)))) :`true` (`self.SubItems`)) null)
          (`self.K2_DestroyActor`))))
    (:`Remote`
      (`self.K2_DestroyActor`))))

(fn `UserConstructionScript`
  (bind _item_id (`self.Item ID`))
  (bind _staticmesh (`self.StaticMesh`))
  (bind (_relativelocation_x _relativelocation_y) (`KismetMathLibrary.BreakVector` (`SceneComponent.RelativeLocation` _staticmesh)))
  (if (`self.Update Mesh On Construct`)
    (`TextRenderComponent.K2_SetText` (`self.TextRender`) (`KismetTextLibrary.Conv_NameToText` _item_id))
    (bind _outitem (`DataRegistrySubsystem.FindCachedItemBP` (make `DataRegistryId` "Items" _item_id))
      (:`Found`
        (`StaticMeshComponent.SetStaticMesh` (`self.StaticMesh`) (`.PickupMesh` (break `InventoryItem` _outitem)))
        (`SceneComponent.K2_SetRelativeLocation` (`self.TextRender`) (`KismetMathLibrary.MakeVector` _relativelocation_x _relativelocation_y (+ (.z (`.Max` (`StaticMeshComponent.GetLocalBounds` _staticmesh))) 20.0)) false false)))))