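; Lite health component for a Character that tracks health, reports damage and death through events, and handles respawn.
; On BeginPlay it spawns optional hit and death effect actors attached to the mesh.
; PointDamage lowers health, clamped from zero to max, then fires damage and death events; a separate helper scales damage by bone.
; Health's RepNotify fires the change event; RestartPlayer uses a server event to destroy the character and restart its controller.
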(event `self.ReceiveBeginPlay`
  (bind _hiteffectclass (`self.HitEffectClass`))
  (bind _deatheffectclass (`self.DeathEffectClass`))
  (bind _ascharacter (cast `Character` (`self.GetOwner`)))
  (set `self.Character` _ascharacter)
  (`|ExecutionSequence`
    (:`then_0`
      (if (`KismetSystemLibrary.IsValidClass` _hiteffectclass)
        (bind _returnvalue (`|SpawnActorFromClass` _hiteffectclass (`KismetMathLibrary.MakeTransform` (0.0 0.0 0.0)) "Undefined" "OverrideRootScale" (`self.GetOwner`) null))
        (`Actor.K2_AttachToComponent` _returnvalue (`Character.Mesh` (`self.Character`)) "None" "KeepRelative" "KeepRelative" "KeepRelative" true)))
    (:`then_1`
      (if (`KismetSystemLibrary.IsValidClass` _deatheffectclass)
        (bind _returnvalue_2 (`|SpawnActorFromClass` _deatheffectclass (`KismetMathLibrary.MakeTransform` (0.0 0.0 0.0)) "Undefined" "OverrideRootScale" (`self.GetOwner`) null))
        (`/Engine/EditorBlueprintResources/StandardMacros.IsValid` _returnvalue_2
          (:`Is Valid`
            (`Actor.K2_AttachToComponent` _returnvalue_2 (`Character.Mesh` (`self.Character`)) "None" "KeepRelative" "KeepRelative" "KeepRelative" true)))))))

(event `RestartPlayer_Server`
  (bind _ascharacter (cast `Character` (`self.GetOwner`)))
  (set `self.ControllerRef` (`Pawn.GetController` _ascharacter))
  (`Actor.K2_DestroyActor` _ascharacter)
  (`GameModeBase.RestartPlayer` (`GameplayStatics.GetGameMode`) (`self.ControllerRef`)))

(fn `Death`
  (`self.IncHealth` (* (`self.Health`) -1.0))
  (`self.Event_OnDeath` 0.0))

(fn `GetCharacter`
  (returns (AsCharacter :type "Character Object Reference"))
  (bind _ascharacter (cast `Character` (`self.GetOwner`)))
  (return _ascharacter))

(fn `IncHealth`
  (params (Value :type "Float (double-precision)"))
  (returns (Health :type "Float (double-precision)"))
  (locals (Local_OldHealth :type "Float (double-precision)" :default 0.0))
  (bind _health (`self.Health`))
  (bind _returnvalue (+ _health (`local.Value`)))
  (set `local.Local_OldHealth` _health)
  (if (> _returnvalue 0.0)
    (set `self.Health` (`KismetMathLibrary.FMin` _returnvalue (`self.MaxHealth`)))
    (else
      (set `self.Health` 0.0)))
  (return (`self.Health`)))

(fn `OnRep_Health`
  (`self.Event_OnHealthChanged`))

(fn `PointDamage`
  (params (Damage :type "Float (single-precision)") (DamageType :type "DamageType Object Reference") (HitLocation :type "Vector Structure") (HitNormal :type "Vector Structure") (HitComponent :type "PrimitiveComponent Object Reference") (BoneName :type Name) (ShotFromDirection :type "Vector Structure") (InstigatedBy :type "Controller Object Reference") (DamageCauser :type "Actor Object Reference") (HitInfo :type "HitResult Structure (by ref)"))
  (if (> (`self.Health`) 0.0)
    (`self.IncHealth` (* (`local.Damage`) -1.0))
    (`self.Event_OnDamageTaken` (`local.Damage`) (`local.ShotFromDirection`) (`local.InstigatedBy`) (`local.HitInfo`) (`local.DamageCauser`) (`local.DamageType`))
    (if (<= (`self.Health`) 0.0)
      (`self.Event_OnDeath` (`local.Damage`) (`local.ShotFromDirection`) (`local.InstigatedBy`) (`local.HitInfo`) (`local.DamageCauser`) (`local.DamageType`)))))

(fn `ResetDamageByBone`
  (params (BoneName :type Name) (Damage :type "Float (double-precision)"))
  (returns (`Return Value` :type "Float (double-precision)"))
  (locals (DamageScale :type "Float (double-precision)"))
  (`|ExecutionSequence`
    (:`then_0`
      (switch `name` (`KismetStringLibrary.Conv_StringToName` (`KismetStringLibrary.ToLower` (`KismetStringLibrary.Conv_NameToString` (`local.BoneName`))))
        (:`Default`
          (set `local.DamageScale` 0.5))
        (:`head`
          (set `local.DamageScale` 3.0))
        (:`pelvis`
          (set `local.DamageScale` 1.0 :!label _label))
        (:`spine_01`
          (goto _label))
        (:`spine_02`
          (goto _label))
        (:`spine_03`
          (goto _label))
        (:`spine_04`
          (goto _label))
        (:`spine_05`
          (goto _label))))
    (:`then_1`
      (return (* (`local.Damage`) (`local.DamageScale`))))))

(fn `RestartPlayer`
  (`self.RestartPlayer_Server`))